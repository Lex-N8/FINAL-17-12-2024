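; BP_EnemyAI is an enemy character that patrols by walking forward and turning around at obstacles, killing the player on contact.
; MoveFoward, not called here, adds forward movement input; WallDetector overlap begins and LedgeDetector overlap ends both call TurnChar for a 180-degree flip.
; Overlapping Teletransportar1 sends MorirMessage to actors implementing the BP_Daño interface.
; Player-chasing logic is unfinished: FollowPlayer is empty and the AIMoveTo chain is disconnected.
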(event `MoveFoward`
  ;[1 1 1] "Seguir al personaje"
  (`self.AddMovementInput` (`self.GetActorForwardVector`)))

(event `self.ReceiveTick`
  (params (DeltaSeconds :type "Float (single-precision)")))

(event `FollowPlayer`
  ;[1 1 1] "Seguir al personaje"
)

(event `self.WallDetector.OnComponentBeginOverlap`
  (params (OverlappedComponent :type "PrimitiveComponent Object Reference") (OtherActor :type "Actor Object Reference") (OtherComp :type "PrimitiveComponent Object Reference") (OtherBodyIndex :type Integer) (bFromSweep :type Boolean) (SweepResult :type "HitResult Structure (by ref)"))
  ;[1 1 1] Turn Char cuando "Wall Detector" sienta una pared
  (`self.TurnChar`))

(event `self.LedgeDetector.OnComponentEndOverlap`
  (params (OverlappedComponent :type "PrimitiveComponent Object Reference") (OtherActor :type "Actor Object Reference") (OtherComp :type "PrimitiveComponent Object Reference") (OtherBodyIndex :type Integer))
  ;[1 1 1] Turn Char cuando Ledge Detector no sienta el piso
  (`self.TurnChar`))

(event `self.Teletransportar1.OnComponentBeginOverlap`
  (params (OverlappedComponent :type "PrimitiveComponent Object Reference") (OtherActor :type "Actor Object Reference") (OtherComp :type "PrimitiveComponent Object Reference") (OtherBodyIndex :type Integer) (bFromSweep :type Boolean) (SweepResult :type "HitResult Structure (by ref)"))
  ;[1 1 1] "Matar" "Atrapar" al personaje
  (if (`KismetSystemLibrary.DoesImplementInterface` OtherActor "/Game/Interface/BP_Daño.BP_Daño_C")
    (message `/Game/Interface/BP_Daño.Morir` OtherActor)))

(fn `TurnChar`
  (`self.K2_SetActorRotation` (`KismetMathLibrary.ComposeRotators` (`self.K2_GetActorRotation`) (struct :`Yaw` 180.0))))

(fn `UserConstructionScript`)