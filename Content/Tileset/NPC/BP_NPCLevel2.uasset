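; Level 2 NPC that shows a text prompt and runs a voiced, multi-line dialogue with the player character.
; Entering its box reveals the text and creates a fresh W_Dialogue widget; leaving hides and removes them.
; EventDialogue, not called within this graph, passes the Text array to the widget, plays the matching Voice sound and advances TextRow, removing the widget after the last line.
; A DoOnce gates each advance and resets immediately afterward.
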(event `self.Box.OnComponentBeginOverlap`
  (params (OverlappedComponent :type "PrimitiveComponent Object Reference") (OtherActor :type "Actor Object Reference") (OtherComp :type "PrimitiveComponent Object Reference") (OtherBodyIndex :type Integer) (bFromSweep :type Boolean) (SweepResult :type "HitResult Structure (by ref)"))
  ;[1 1 1] Ocultar el texto solo si el jugador se acerca
  (cast `/Game/Characters/BP_PersonajeTP` OtherActor)
  (`SceneComponent.SetHiddenInGame` (`self.TextRender`) false false)
  (bind _returnvalue (`|CreateWidget` "/Game/Tileset/NPC/W_Dialogue.W_Dialogue_C"))
  (bind _output_get (set `self.DIalogueUI` _returnvalue))
  (`UserWidget.AddToViewport` _output_get 0))

(event `self.Box.OnComponentEndOverlap`
  (params (OverlappedComponent :type "PrimitiveComponent Object Reference") (OtherActor :type "Actor Object Reference") (OtherComp :type "PrimitiveComponent Object Reference") (OtherBodyIndex :type Integer))
  (bind _dialogueui (`self.DIalogueUI`))
  ;[1 1 1] Ocultar el texto solo si el jugador se acerca
  (cast `/Game/Characters/BP_PersonajeTP` OtherActor)
  (`SceneComponent.SetHiddenInGame` (`self.TextRender`) true false)
  (`/Engine/EditorBlueprintResources/StandardMacros.IsValid` _dialogueui
    (:`Is Valid`
      (`Widget.RemoveFromParent` _dialogueui))))

(event `/Game/Tileset/NPC/DialogueInterface.EventDialogue`
  (bind _dialogueui (`self.DIalogueUI`))
  (bind _dialogueui_2 (`self.DIalogueUI`))
  (bind _returnvalue (+ (`/Game/Tileset/NPC/W_Dialogue.TextRow` (`self.DIalogueUI`)) 1))
  ;[1 1 1] Reset de dialogo y do once de este
  (`/Engine/EditorBlueprintResources/StandardMacros.DoOnce` false :!label _label
    (:`Completed`
      (set `/Game/Tileset/NPC/W_Dialogue.Text` (`self.Text`) _dialogueui_2)
      (`Widget.SetVisibility` (`/Game/Tileset/NPC/W_Dialogue.TextDialogue` _dialogueui_2) "Visible")
      (`Widget.SetVisibility` (`/Game/Tileset/NPC/W_Dialogue.DialogueBorder` _dialogueui_2) "Visible")
      ;[1 1 1] Sonido para cada dialogo
      (`GameplayStatics.PlaySound2D` (`|GetArrayItem` (`self.Voice`) (+ (`/Game/Tileset/NPC/W_Dialogue.TextRow` (`self.DIalogueUI`)) 1)) 1.0 1.0 0.0 null null)
      ;[1 1 1] Texto del dialogo, con array para modificar y agregar varios con reset y do once
      (if (> _returnvalue (- (`KismetArrayLibrary.Array_Length` (`self.Text`)) 1))
        (`Widget.RemoveFromParent` _dialogueui)
        (`self.ResetDoOnce`)
        (else
          (set `/Game/Tileset/NPC/W_Dialogue.TextRow` _returnvalue _dialogueui)
          (`self.ResetDoOnce`))))))

(event `ResetDoOnce`
  ;[1 1 1] Reset de dialogo y do once de este
  (goto _label :!via `Reset`))

(fn `UserConstructionScript`)